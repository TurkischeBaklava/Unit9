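; BP_Telly is a television actor with media playback and an on-screen control widget shown by proximity.
; At BeginPlay it constructs a new MediaPlayer from the assigned one's class and binds it to a media texture and an added sound component.
; Entering the box collision shows the widget, mouse cursor and Game and UI input mode.
; Leaving hides them and restores game-only input, with no filter on the overlapping actor.
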(event OnComponentBeginOverlap(BoxCollision)
  (params (OverlappedComponent :type Primitive%20Component%20Object%20Reference) (OtherActor :type Actor%20Object%20Reference) (OtherComp :type Primitive%20Component%20Object%20Reference) (OtherBodyIndex :type Integer) (bFromSweep :type Boolean) (SweepResult :type Hit%20Result%20Structure%20%28by%20ref%29))
  (bind _returnvalue (Class|UELTv|GetControllerOfActor OtherActor))
  (Input|DisableInput OtherActor _returnvalue)
  (Class|UELTv|SetMediaPlayerWidgetVisibility true)
  ;[1 1 1] UI
  (Input|SetInputModeGameandUI _returnvalue 0 "DoNotLock" true)
  (Variables|/Script/Engine.PlayerController|SetbShowMouseCursor _returnvalue true)
  (Input|EnableInput OtherActor _returnvalue))

(event OnComponentEndOverlap(BoxCollision)
  (params (OverlappedComponent :type Primitive%20Component%20Object%20Reference) (OtherActor :type Actor%20Object%20Reference) (OtherComp :type Primitive%20Component%20Object%20Reference) (OtherBodyIndex :type Integer))
  (bind _returnvalue (Class|UELTv|GetControllerOfActor OtherActor))
  (Class|UELTv|SetMediaPlayerWidgetVisibility false)
  (Input|SetInputModeGameOnly _returnvalue)
  (Variables|/Script/Engine.PlayerController|SetbShowMouseCursor _returnvalue false))

(event EventBeginPlay
  (bind _mediaplayer (Variables|Default|GetMediaPlayer)
    (:then
      (bind _returnvalue (Game|ConstructObjectfromClass (Utilities|GetClass _mediaplayer) self))
      (bind _output_get (Variables|Default|SetMediaPlayer _returnvalue))
      (Media|MediaSoundComponent|SetMediaPlayer (Variables|Default|GetNewMediaTexture) _output_get)
      (bind _returnvalue_2 (AddComponent|AddMediaSoundComponent false))
      (Media|MediaSoundComponent|SetMediaPlayer _returnvalue_2 _output_get))
    (:else)))

(fn ConstructionScript)

(fn GetPlayerCharacter
  (return (.AsThird%20Person%20Character (Utilities|Casting|CastToThirdPersonCharacter (Game|Player|GetPlayerPawn 0)))))